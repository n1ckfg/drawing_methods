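; BP_MousePos converts the mouse cursor of player 0 into a world-space position every tick and stores it in MousePos.
; With MapToXZ set, it intersects the deprojected cursor ray with the world Z=0 plane, which is the XY plane despite the flag's name.
; Otherwise, it takes the point Ybounds units along the ray from the deprojected origin.
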(event EventTick
  (params (DeltaSeconds :type Float%20%28single-precision%29))
  (bind _returnvalue (Game|GetPlayerController 0))
  (bind (_worldlocation _worlddirection) (Game|Player|ConvertMouseLocationToWorldSpace _returnvalue))
  (if (Variables|Default|GetMapToXZ)
    (Variables|Default|SetMousePos (+ _worldlocation (* (* _worlddirection (/ (.Z (Math|Vector|BreakVector _worldlocation)) (.Z (Math|Vector|BreakVector _worlddirection)))) -1.0)))
    (else
      (Variables|Default|SetMousePos (+ (* _worlddirection (Variables|Default|GetYbounds)) _worldlocation)))))

(fn ConstructionScript)