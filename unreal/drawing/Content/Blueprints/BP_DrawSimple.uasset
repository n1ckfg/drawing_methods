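; BP_DrawSimple is a drawing actor that creates brush strokes as child actors, one per BeginDrawing call.
; BeginDrawing adds the child actor, caches it as a BP_BrushStrokeSimple and opens a gate on Tick.
; While the gate is open, each tick writes NewPoint into the stroke's StrokePoints at an incrementing index and calls Rebuild.
; EndDrawing resets the index and closes the gate.
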(event Custom|BeginDrawing
  (bind _returnvalue (AddComponent|AddChildActorComponent false))
  (bind _asbp_brush_stroke_simple (Utilities|Casting|CastToBP_BrushStrokeSimple (Variables|/Script/Engine.ChildActorComponent|GetChildActor _returnvalue)))
  (Utilities|FlowControl|Gate true) ; enters at Open
)

(event Custom|EndDrawing
  (Variables|Default|SetDrawPointIndex 0)
  (Utilities|FlowControl|Gate true) ; enters at Close
)

(event EventTick
  (params (DeltaSeconds :type Float%20%28single-precision%29))
  (Utilities|FlowControl|Gate true
    (:Exit
      (Utilities|Array|SetArrayElem (stale _output_get) (Variables|Default|GetDrawPointIndex) (Variables|Default|GetNewPoint) true)
      (bind _result (Math|Integer|IncrementInt (Variables|Default|GetDrawPointIndex))
        (:%20%20
          (Variables|Default|SetDrawPointIndex _result)
          (bind _output_get (Variables|/Game/Blueprints/BP_BrushStrokeSimple.BP_BrushStrokeSimple_C|SetStrokePoints (stale Custom|BeginDrawing _asbp_brush_stroke_simple) (Variables|/Game/Blueprints/BP_BrushStrokeSimple.BP_BrushStrokeSimple_C|GetStrokePoints (stale Custom|BeginDrawing _asbp_brush_stroke_simple))))
          (Default|Rebuild (stale Custom|BeginDrawing _asbp_brush_stroke_simple)))))))

(fn ConstructionScript)