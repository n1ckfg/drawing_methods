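; BP_BrushStrokeSimple is a simple brush stroke that renders its StrokePoints as a low-poly cylinder strip.
; On BeginPlay, MakeCylinderStrip adds a child actor and casts it to BP_Cylinder, then sets its line points, four-sided profile, radius and default Latk material before refreshing it.
; The Rebuild event re-enters after the spawn and cast, reapplying those settings to the existing cylinder.
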(event Custom|Rebuild
  (Utilities|MakeCylinderStrip) ; enters at Rebuild
)

(event EventBeginPlay
  (Utilities|MakeCylinderStrip))

(fn ConstructionScript)